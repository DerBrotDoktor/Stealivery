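; BP_TurtleShell is a turtle shell item actor for the DeliveryDriver game, with sounds for shooting, rolling and hitting.
; On BeginPlay it plays the shoot and roll sounds, waits for DestroyTime, then stops the roll sound and destroys itself.
; Collision hit events play the hit sound, and the graph contains no movement or damage logic.
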(event `self.ReceiveBeginPlay`
  (`AudioComponent.Play` (`self.BallShootSFX`) 0.0)
  (`AudioComponent.Play` (`self.BallRollSFX`) 0.0)
  (`KismetSystemLibrary.Delay` (`self.DestroyTime`))
  (`AudioComponent.Stop` (`self.BallRollSFX`))
  (`self.K2_DestroyActor`))

(event `self.Collision.OnComponentHit`
  (params (HitComponent :type "PrimitiveComponent Object Reference") (OtherActor :type "Actor Object Reference") (OtherComp :type "PrimitiveComponent Object Reference") (NormalImpulse :type "Vector Structure") (Hit :type "HitResult Structure (by ref)"))
  (`AudioComponent.Play` (`self.BallHitSFX`) 0.0))

(fn `UserConstructionScript`)