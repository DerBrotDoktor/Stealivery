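; BP_ItemSpawner is a respawning pickup point that spawns a random item from its Items list at its SpawnPoint.
; On BeginPlay and after each Cooldown timer, SpawnItem creates the item, caches its type and enables overlap events on the Area.
; PickUpItem disables those overlaps, destroys the item, restarts the VFX, plays a sound and schedules the next spawn.
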(event `self.ReceiveBeginPlay`
  (`self.SpawnItem`))

(event `PickUpItem`
  (set `PrimitiveComponent.bGenerateOverlapEvents` false (`self.Area`))
  (`self.K2_DestroyActor` (`self.SpawnedActor`))
  (`KismetSystemLibrary.K2_SetTimerDelegate` (delegate `SpawnItem`) (`self.Cooldown`))
  (`NiagaraComponent.ResetSystem` (`self.VFX`))
  (`AudioComponent.Play` (`self.SFX`) 0.0))

(event `SpawnItem`
  (bind _outitem (`KismetArrayLibrary.Array_Random` (`self.Items`)))
  (bind _returnvalue (`|SpawnActorFromClass` _outitem (`KismetMathLibrary.MakeTransform` (`SceneComponent.K2_GetComponentLocation` (`self.SpawnPoint`))) "Undefined" "MultiplyWithRoot" null null))
  (bind _output_get (set `self.SpawnedActor` _returnvalue))
  (set `self.ItemType` (`/Game/DeliveryDriver/Core/Items/BP_BaseItem.Type` _output_get))
  (set `PrimitiveComponent.bGenerateOverlapEvents` true (`self.Area`)))

(fn `UserConstructionScript`)