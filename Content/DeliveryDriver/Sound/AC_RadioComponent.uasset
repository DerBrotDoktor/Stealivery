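; Actor component for a car-radio style music player that plays random 2D songs from a list with fade-outs.
; SelectNewSong rerolls until the pick differs from the current song, and TryFadeOutOldSong fades out any playing one.
; A self-repeating chain spawns each song and calls ChangeSong shortly before it ends.
; BeginPlay and ChangeSong are both unwired, so this playback chain never runs as it stands.
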(event `self.ReceiveBeginPlay`)

(event `ChangeSong`)

(fn `SelectNewSong`
  (returns (SelectedSong :type "SoundBase Object Reference"))
  (locals (ProvisionalSong :type "SoundBase Object Reference"))
  (bind _songlist (`self.SongList`))
  (set `local.ProvisionalSong` (`|GetArrayItem` _songlist (`KismetMathLibrary.RandomIntegerInRange` 0 (`KismetArrayLibrary.Array_LastIndex` _songlist))) :!label _label)
  (if (== (`self.CurrentSongSoundBase`) (`local.ProvisionalSong`))
    (goto _label)
    (else
      (return (`local.ProvisionalSong`)))))

(fn `TryFadeOutOldSong`
  (returns (IsFading :type Boolean))
  (bind _currentsongref (`self.CurrentSongRef`)
    (:`then`
      (`AudioComponent.FadeOut` _currentsongref (`self.FadeDuration`) 0.0 "Linear")
      (return true))
    (:`else`
      (return false))))