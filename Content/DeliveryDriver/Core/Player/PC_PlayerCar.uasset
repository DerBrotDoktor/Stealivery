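; Player controller for the player car in DeliveryDriver, linking a player ID to the possessed car and showing the start countdown.
; On possess it passes the ID to the BP_BasePlayerCar, caches that pawn and disables its input.
; SetPlayerID updates both the controller and cached car, with debug prints.
; Timer events create, update and remove a countdown widget on that player's own screen.
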(event `self.ReceivePossess`
  (params (PossessedPawn :type "Pawn Object Reference"))
  ; On Possesss
  (bind _asbp_base_player_car (cast `/Game/DeliveryDriver/Core/Player/BP_BasePlayerCar` PossessedPawn))
  (`/Game/DeliveryDriver/Core/Player/BP_BasePlayerCar.OnSetPlayerID` _asbp_base_player_car (`self.PlayerID`))
  (set `self.PosseedPawn` _asbp_base_player_car)
  (`/Game/DeliveryDriver/Core/Player/BP_BasePlayerCar.SetInput` _asbp_base_player_car false))

(event `OnCreateStartTimer`
  ; Start Countdown
  (`/Engine/EditorBlueprintResources/StandardMacros.IsValid` (`self.StartCountdown`)
    (:`Is Valid`
      _)
    (:`Is Not Valid`
      (`self.OnDestroyStartTimer`)))
  (bind _returnvalue (`|CreateWidget` "/Game/DeliveryDriver/UI/WBP_StartCountdown.WBP_StartCountdown_C" self))
  (bind _output_get (set `self.StartCountdown` _returnvalue))
  (`UserWidget.AddToPlayerScreen` _output_get 0))

(event `OnUpdateStartTimer`
  (params (Time :type Integer))
  ; Start Countdown
  (`/Engine/EditorBlueprintResources/StandardMacros.IsValid` (`self.StartCountdown`)
    (:`Is Valid`
      (`/Game/DeliveryDriver/UI/WBP_StartCountdown.SetTime` (`self.StartCountdown`) Time))))

(event `OnDestroyStartTimer`
  ; Start Countdown
  (`/Engine/EditorBlueprintResources/StandardMacros.IsValid` (`self.StartCountdown`)
    (:`Is Valid`
      (`Widget.RemoveFromParent` (`self.StartCountdown`))
      (set `self.StartCountdown` null))))

(fn `SetPlayerID`
  (params (ID :type Integer))
  (bind _posseedpawn (`self.PosseedPawn`))
  (set `self.PlayerID` ID)
  (`/Engine/EditorBlueprintResources/StandardMacros.IsValid` _posseedpawn
    (:`Is Valid`
      (bind _asbp_base_player_car (cast `/Game/DeliveryDriver/Core/Player/BP_BasePlayerCar` _posseedpawn))
      (bind _output_get (set `/Game/DeliveryDriver/Core/Player/BP_BasePlayerCar.PlayerID` (`self.PlayerID`) _asbp_base_player_car))
      (`KismetSystemLibrary.PrintString` (`KismetStringLibrary.Concat_StrStr` "PlayerController" "set Player ID:" (`KismetStringLibrary.Conv_IntToString` _output_get)))
      (return))
    (:`Is Not Valid`
      (`KismetSystemLibrary.PrintString` "Player controller possessed pawn invalid")
      (return))))

(fn `UserConstructionScript`)