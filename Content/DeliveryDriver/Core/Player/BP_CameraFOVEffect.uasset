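; BP_CameraFOVEffect changes the player car's camera field of view as it drives, blending between a default and a target value.
; On BeginPlay it caches its BP_BasePlayerCar owner and starts a looping timer for the update.
; While moving forward, the blend follows normalized engine rotation speed below 70%, otherwise normalized forward speed.
; FInterpToConstant eases the FOV toward that value, returning to default when not moving forward.
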(event `self.ReceiveBeginPlay`
  (bind _asbp_base_player_car (cast `/Game/DeliveryDriver/Core/Player/BP_BasePlayerCar` (`self.GetOwner`))
    (:`then`
      (set `self.Character` _asbp_base_player_car)
      (bind _returnvalue (`KismetSystemLibrary.K2_SetTimerDelegate` (delegate `OnUpdateFOV`) (`self.UpdateTimerTime`) true))
      (set `self.UpdateTimerHandle` _returnvalue))
    (:`CastFailed`
      (`KismetSystemLibrary.PrintString` "Invalid Camera FOV Effect Owner" true true (struct :`R` 1.0 :`A` 1.0)))))

(event `OnUpdateFOV`
  (bind _deliveryvehiclemovementcomponent (`/Game/DeliveryDriver/Core/Player/BP_BasePlayerCar.DeliveryVehicleMovementComponent` (`self.Character`)))
  (bind _camera (`/Game/DeliveryDriver/Core/Player/BP_BasePlayerCar.Camera` (`self.Character`)))
  (bind _returnvalue (`KismetMathLibrary.NormalizeToRange` (`ChaosWheeledVehicleMovementComponent.GetEngineRotationSpeed` _deliveryvehiclemovementcomponent) 0.0 (`ChaosWheeledVehicleMovementComponent.GetEngineMaxRotationSpeed` _deliveryvehiclemovementcomponent)))
  (if (> (`ChaosVehicleMovementComponent.GetForwardSpeed` _deliveryvehiclemovementcomponent) 1.0)
    (set `self.ForwardAlpha` (select `bool` (< _returnvalue 0.7) :`false` (`KismetMathLibrary.NormalizeToRange` (`ChaosVehicleMovementComponent.GetForwardSpeed` _deliveryvehiclemovementcomponent) 0.0 (`MovementComponent.GetMaxSpeed` _deliveryvehiclemovementcomponent)) :`true` _returnvalue))
    (else
      (set `self.ForwardAlpha` 0.0)))
  (`CameraComponent.SetFieldOfView` _camera (`KismetMathLibrary.FInterpTo_Constant` (`CameraComponent.FieldOfView` _camera) (`KismetMathLibrary.Lerp` (`self.FOVDefault`) (`self.FOVTarget`) (`self.ForwardAlpha`)) (`GameplayStatics.GetWorldDeltaSeconds`) (`self.InterpSpeed`))))