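; Base level actor for the delivery driving game that runs the match flow from start countdown through timed play to the finish screen.
; StartGame polls each tick until multiple player controllers exist, then starts music, locks car input for a three-second countdown and notifies the IGameManager actor.
; Tick drives the HUD timer, which OnAddTime can extend.
; At zero, GameFinished pauses, shows the finish widget and opens the finish level after a delay.
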(event `self.ReceiveBeginPlay`
  ;[0.6 0.15 0.15 0.5] Being Play / Setup
  (set `self.LevelTimeLeft` (`KismetMathLibrary.Conv_IntToDouble` (`self.LevelTime`)))
  (bind _returnvalue (`|CreateWidget` "/Game/DeliveryDriver/UI/WBP_PlayerHUD.WBP_PlayerHUD_C"))
  (bind _output_get (set `self.TimeUI` _returnvalue))
  (`/Game/DeliveryDriver/UI/WBP_PlayerHUD.SetTimer` _output_get (`self.LevelTimeLeft`))
  (`UserWidget.AddToViewport` _output_get 0)
  (`KismetSystemLibrary.DelayUntilNextTick`)
  (`self.StartGame`))

(event `StartGame`
  ; StartGame
  (bind _outactors (`GameplayStatics.GetAllActorsOfClass` "/Game/DeliveryDriver/Core/Player/PC_PlayerCar.PC_PlayerCar_C" :!label _label))
  (if (> (`KismetArrayLibrary.Array_Length` _outactors) 1)
    (`|ExecutionSequence`
      (:`then_0`
        (bind _asgi_game_instance (cast `/Game/DeliveryDriver/Core/Game/GI_GameInstance` (`GameplayStatics.GetGameInstance`)))
        (`/Game/DeliveryDriver/Core/Game/GI_GameInstance.PlayMusic` _asgi_game_instance "/Game/DeliveryDriver/Sound/SC_Radio.SC_Radio"))
      (:`then_1`
        (bind _outactors_2 (`GameplayStatics.GetAllActorsOfClass` "/Game/DeliveryDriver/Core/Player/BP_BasePlayerCar.BP_BasePlayerCar_C"))
        (for _array_element _outactors_2
          (`/Game/DeliveryDriver/Core/Player/BP_BasePlayerCar.SetInput` _array_element false)))
      (:`then_2`
        (for _array_element_2 _outactors
          (`/Game/DeliveryDriver/Core/Player/PC_PlayerCar.OnCreateStartTimer` _array_element_2))
        (bind _counter (`/Engine/EditorBlueprintResources/StandardMacros.Do N` 3 :!label _label_2)
          (:`Exit`
            (for _array_element_3 _outactors
              (bind _returnvalue (- 4 _counter))
              (`/Game/DeliveryDriver/Core/Player/PC_PlayerCar.OnUpdateStartTimer` _array_element_3 _returnvalue))
            (`KismetSystemLibrary.PrintString` (`KismetStringLibrary.Conv_IntToString` _returnvalue))
            (`KismetSystemLibrary.Delay` 1.0)
            (if (< _counter 3)
              (goto _label_2)
              (else
                (for _array_element_4 _outactors
                  (`/Game/DeliveryDriver/Core/Player/PC_PlayerCar.OnDestroyStartTimer` _array_element_4))
                (bind _outactors_3 (`GameplayStatics.GetAllActorsWithInterface` "/Game/DeliveryDriver/Core/Game/IGameManager.IGameManager_C"))
                (message `/Game/DeliveryDriver/Core/Game/IGameManager.StartGame` (`|GetArrayItem` _outactors_3))
                (`KismetSystemLibrary.PrintString` "Start Game" true true (struct :`R` 1.0 :`B` 0.781608 :`A` 1.0))
                (bind _outactors_4 (`GameplayStatics.GetAllActorsOfClass` "/Game/DeliveryDriver/Core/Player/BP_BasePlayerCar.BP_BasePlayerCar_C"))
                (for _array_element_5 _outactors_4
                  (`/Game/DeliveryDriver/Core/Player/BP_BasePlayerCar.SetInput` _array_element_5 true))
                (`self.OnEnableTimer`)))))))
    (else
      (`KismetSystemLibrary.DelayUntilNextTick`)
      (goto _label))))

(event `self.ReceiveTick`
  (params (DeltaSeconds :type "Float (single-precision)"))
  ; Timer
  (if (and (`self.bShouldUpdateTime`) (not (`GameplayStatics.IsGamePaused`)))
    (bind _output_get (set `self.LevelTimeLeft` (- (`self.LevelTimeLeft`) DeltaSeconds)))
    (`/Game/DeliveryDriver/UI/WBP_PlayerHUD.SetTimer` (`self.TimeUI`) (`KismetMathLibrary.Conv_IntToDouble` (`KismetMathLibrary.FTrunc` _output_get)))
    ;; Out of Time
    (if (<= (`self.LevelTimeLeft`) 0.0)
      (`self.GameFinished`))))

(event `OnEnableTimer`
  ; Timer
  (`/Engine/EditorBlueprintResources/StandardMacros.IsValid` (`self.TimeUI`)
    (:`Is Valid`
      (set `self.bShouldUpdateTime` true)
      (bind _returnvalue (`|CreateWidget` "/Game/DeliveryDriver/UI/MiniMap/WBP_MiniMap.WBP_MiniMap_C"))
      (bind _outactors (`GameplayStatics.GetAllActorsOfClass` "/Game/DeliveryDriver/Player/Blueprints/BP_PlayerCar.BP_PlayerCar_C"))
      (for _array_element _outactors
        (`/Game/DeliveryDriver/Player/Blueprints/BP_PlayerCar.SetMiniMapIcons` _array_element))
      (`UserWidget.AddToViewport` _returnvalue 0))))

(event `OnDisableTimer`
  ; Timer
  (set `self.bShouldUpdateTime` false))

(event `OnAddTime`
  (params (Time :type Integer))
  ; Timer
  (set `self.LevelTimeLeft` (+ Time (`self.LevelTimeLeft`))))

(event `GameFinished`
  ; Game Finished
  (`/Engine/EditorBlueprintResources/StandardMacros.DoOnce` false
    (:`Completed`
      (`GameplayStatics.SetGamePaused` true)
      (set `self.bShouldUpdateTime` false)
      (`Widget.RemoveFromParent` (`self.TimeUI`))
      (bind _returnvalue (`|CreateWidget` "/Game/DeliveryDriver/UI/WBP_Finish.WBP_Finish_C"))
      (`UserWidget.AddToViewport` _returnvalue 0)
      (`GameplayStatics.PlaySound2D` "/Game/DeliveryDriver/Sound/Sounds/A_Finish.A_Finish" 1.0 1.0 0.0 null null)
      (`KismetSystemLibrary.Delay` (`self.FinishDisplayTime`))
      (`GameplayStatics.OpenLevelBySoftObjectPtr` "/Game/DeliveryDriver/Maps/FinishScreen.FinishScreen"))))

(fn `UserConstructionScript`)