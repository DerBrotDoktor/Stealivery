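; BP_BaseGameStart is a base start-zone actor for Delivery Driver that counts player cars inside its Area volume.
; On BeginPlay it caches NumPlayers from GM_Game, and each car entering compares the overlapping car count against it.
; The branch for all players present is empty, and the end-overlap decrement has no lasting effect.
; The actor destroys itself when OnGameStarted fires.
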(event `self.ReceiveBeginPlay`
  (bind _asgm_game (cast `/Game/DeliveryDriver/Core/GameModes/GM_Game` (`GameplayStatics.GetGameMode`)))
  (set `self.Num Players` (`/Game/DeliveryDriver/Core/GameModes/GM_Game.NumPlayers` _asgm_game)))

(event `self.Area.OnComponentBeginOverlap`
  (params (OverlappedComponent :type "PrimitiveComponent Object Reference") (OtherActor :type "Actor Object Reference") (OtherComp :type "PrimitiveComponent Object Reference") (OtherBodyIndex :type Integer) (bFromSweep :type Boolean) (SweepResult :type "HitResult Structure (by ref)"))
  (cast `/Game/DeliveryDriver/Core/Player/BP_BasePlayerCar` OtherActor)
  (if (<= (`self.Num Players`) (`KismetArrayLibrary.Array_Length` (`PrimitiveComponent.GetOverlappingActors` (`self.Area`) "/Game/DeliveryDriver/Core/Player/BP_BasePlayerCar.BP_BasePlayerCar_C")))
    _))

(event `self.Area.OnComponentEndOverlap`
  (params (OverlappedComponent :type "PrimitiveComponent Object Reference") (OtherActor :type "Actor Object Reference") (OtherComp :type "PrimitiveComponent Object Reference") (OtherBodyIndex :type Integer))
  (cast `/Game/DeliveryDriver/Core/Player/BP_BasePlayerCar` OtherActor)
  (bind _result (`/Engine/EditorBlueprintResources/StandardMacros.DecrementInt` (`KismetArrayLibrary.Array_Length` (`PrimitiveComponent.GetOverlappingActors` (`self.Area`) "/Game/DeliveryDriver/Core/Player/BP_BasePlayerCar.BP_BasePlayerCar_C")))))

(event `OnGameStarted`
  (`self.K2_DestroyActor`))

(fn `UserConstructionScript`)