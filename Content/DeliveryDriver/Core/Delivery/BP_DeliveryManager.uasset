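; Delivery manager that runs the pickup and drop-off loop for player cars in the delivery driving game.
; StartGame enables a random non-repeating spawn and picks a target beyond a minimum distance, falling back to any.
; A None/Spawn/Target state follows collection and part-counted completion, respawning after a cooldown.
; It also reroutes active deliveries with a cooldown and steers each car's arrow to spawn, target, carrying car or delivery actor.
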(event `self.ReceiveBeginPlay`
  ;[0.6 0.15 0.15 0.5] Begin Play
  (bind _outactors (`GameplayStatics.GetAllActorsOfClass` "/Game/DeliveryDriver/Core/Delivery/BP_BaseDeliverySpawn.BP_BaseDeliverySpawn_C"))
  (set `self.DeliverySpawns` _outactors)
  (bind _outactors_2 (`GameplayStatics.GetAllActorsOfClass` "/Game/DeliveryDriver/Core/Delivery/BP_BaseDeliveryTarget.BP_BaseDeliveryTarget_C"))
  (set `self.DeliverytTargets` _outactors_2))

(event `OnDeliveryFinished`
  ; Delivery Finished
  (set `self.State` "NewEnumerator0")
  (`KismetSystemLibrary.Delay` (`self.DeliveryCooldown`))
  (set `self.CurrentDeliverdParts` 0)
  (`self.SpawnNewDelivery`))

(event `OnDeliveryCollected`
  (params (Target :type "/Game/DeliveryDriver/Core/Delivery/BP_BaseDeliveryTarget Object Reference"))
  ; Delivery Collected
  (`/Game/DeliveryDriver/Core/Delivery/BP_BaseDeliverySpawn.Disable` (`self.CurrentDeliverySpawn`))
  (`/Game/DeliveryDriver/Core/Delivery/BP_BaseDeliveryTarget.Enable` Target (struct :`R` 0.342099 :`G` 1.0 :`B` 0.744321 :`A` 0.481))
  (set `self.CurrentTargetPosition` (`SceneComponent.K2_GetComponentLocation` (`Actor.RootComponent` Target)))
  (set `self.State` "NewEnumerator2"))

(event `SpawnNewDelivery`
  (bind _currentdeliveryspawn (`self.CurrentDeliverySpawn`))
  (bind _returnvalue (`KismetArrayLibrary.Array_Length` (`self.DeliverySpawns`)))
  ; New Delivery
  (bind (_outitem _outindex) (`KismetArrayLibrary.Array_Random` (`self.DeliverySpawns`)))
  (if (!= _outitem (`self.LastDeliverySpawn`))
    (bind _output_get (set `self.CurrentDeliverySpawn` _outitem :!label _label))
    (set `self.LastDeliverySpawn` _output_get)
    (elif (< _returnvalue 2)
      (goto _label)
      (else
        (bind _result (`/Engine/EditorBlueprintResources/StandardMacros.IncrementInt` _outindex)
          (:`  `
            (bind _output_get_2 (set `self.CurrentDeliverySpawn` (`|GetArrayItem` (`self.DeliverySpawns`) (`KismetMathLibrary.Wrap` _result 0 (- _returnvalue 1)))))
            (set `self.LastDeliverySpawn` _output_get_2))))))
  (bind _outputpin (`self.NewTarget` true (`SceneComponent.K2_GetComponentLocation` (`/Game/DeliveryDriver/Core/Delivery/BP_BaseDeliverySpawn.DefaultSceneRoot` (`self.CurrentDeliverySpawn`)))))
  (`/Game/DeliveryDriver/Core/Delivery/BP_BaseDeliverySpawn.Enable` :`self` _currentdeliveryspawn :`DeliveryTarget` _outputpin)
  (set `self.CurrentTarget` _outputpin)
  (set `self.CurrentTargetPosition` (`SceneComponent.K2_GetComponentLocation` (`Actor.RootComponent` _currentdeliveryspawn)))
  (set `self.State` "NewEnumerator1"))

(event `/Game/DeliveryDriver/Core/Game/IGameManager.StartGame`
  ; Start Game
  (`/Engine/EditorBlueprintResources/StandardMacros.DoOnce` false
    (:`Completed`
      (set `self.bGameStarted` true)
      (`KismetSystemLibrary.PrintString` "Start Deliveries")
      (bind _outactors (`GameplayStatics.GetAllActorsOfClass` "/Game/DeliveryDriver/Core/Player/BP_BasePlayerCar.BP_BasePlayerCar_C"))
      (set `self.PlayerCars` _outactors)
      (`self.SpawnNewDelivery`))))

(event `ChangeDeliveryTarget`
  (params (MinDistanceStartPoint :type "Vector Structure"))
  (bind _currenttarget (`self.CurrentTarget`))
  ; Change Delivery Target
  (if (`/Game/DeliveryDriver/Core/Delivery/BP_BaseDeliveryTarget.bEnabled` (`self.CurrentTarget`))
    (`/Engine/EditorBlueprintResources/StandardMacros.DoOnce` false :!label _label_2
      (:`Completed`
        (`KismetSystemLibrary.PrintString` "Change Delivery Target")
        (`/Engine/EditorBlueprintResources/StandardMacros.IsValid` _currenttarget
          (:`Is Valid`
            (`/Game/DeliveryDriver/Core/Delivery/BP_BaseDeliveryTarget.Disable` _currenttarget))
          (:`Is Not Valid`
            _))
        (bind _outputpin (`self.NewTarget` true MinDistanceStartPoint))
        (bind _outactors (`GameplayStatics.GetAllActorsOfClass` "/Game/DeliveryDriver/Core/Delivery/BP_BaseDelivery.BP_BaseDelivery_C"))
        (for _array_element _outactors
          (bind (_data_target _data_itembp) (break `/Game/DeliveryDriver/Core/Delivery/SDeliveryData` (`/Game/DeliveryDriver/Core/Delivery/BP_BaseDelivery.Data` _array_element)))
          (set `/Game/DeliveryDriver/Core/Delivery/BP_BaseDelivery.Data` (make `/Game/DeliveryDriver/Core/Delivery/SDeliveryData` _outputpin _data_itembp) _array_element))
        (bind _outactors_2 (`GameplayStatics.GetAllActorsOfClass` "/Game/DeliveryDriver/Core/Player/BP_BasePlayerCar.BP_BasePlayerCar_C"))
        (for _array_element_2 _outactors_2
          (bind (_currentdelivery_target _currentdelivery_itembp) (break `/Game/DeliveryDriver/Core/Delivery/SDeliveryData` (`/Game/DeliveryDriver/Core/Player/BP_BasePlayerCar.CurrentDelivery` _array_element_2)))
          (set `/Game/DeliveryDriver/Core/Player/BP_BasePlayerCar.CurrentDelivery` (make `/Game/DeliveryDriver/Core/Delivery/SDeliveryData` _outputpin _currentdelivery_itembp) _array_element_2))
        (`/Game/DeliveryDriver/Core/Delivery/BP_BaseDeliveryTarget.Enable` :`self` _outputpin)
        (set `self.CurrentTarget` _outputpin)
        (set `self.CurrentTargetPosition` (`SceneComponent.K2_GetComponentLocation` (`Actor.RootComponent` _outputpin)))
        (`KismetSystemLibrary.Delay` (`self.ChangeDeliveryCooldown`))
        (`KismetSystemLibrary.PrintString` "cooldown finished" true true (struct :`R` 1.0 :`B` 0.339607 :`A` 1.0))
        (goto _label_2 :!via `Reset`)))))

(fn `DeliverParts`
  (params (Amount :type Integer))
  (returns (DeliveryCompleted :type Boolean))
  (bind _output_get (set `self.CurrentDeliverdParts` (+ Amount (`self.CurrentDeliverdParts`))))
  (bind _returnvalue (>= _output_get (`self.DeliveryParts`)))
  (if _returnvalue
    (`self.OnDeliveryFinished`))
  (return _returnvalue))

(fn `GetDirectionArrowTarget`
  (params (PlayerCar :type "/Game/DeliveryDriver/Core/Player/BP_BasePlayerCar Object Reference"))
  (returns (TargetPosition :type "Vector Structure"))
  (locals (Player :type "/Game/DeliveryDriver/Core/Player/BP_BasePlayerCar Object Reference"))
  (set `local.Player` PlayerCar)
  (switch `/Game/DeliveryDriver/Core/Delivery/EDeliveryManagerState` (`self.State`)
    (:`NewEnumerator0`
      (`/Game/DeliveryDriver/Core/Player/BP_BasePlayerCar.SetDirectionArrowColor` (`local.Player`) false false)
      (return (0.0 0.0 0.0)))
    (:`NewEnumerator1`
      (`/Game/DeliveryDriver/Core/Player/BP_BasePlayerCar.SetDirectionArrowColor` (`local.Player`) true false)
      (return (`SceneComponent.K2_GetComponentLocation` (`Actor.RootComponent` (`self.CurrentDeliverySpawn`)))))
    (:`NewEnumerator2`
      (if (> (`/Game/DeliveryDriver/Core/Player/BP_BasePlayerCar.CurrentDeliveryParts` (`local.Player`)) 0)
        (`/Game/DeliveryDriver/Core/Player/BP_BasePlayerCar.SetDirectionArrowColor` (`local.Player`) true false)
        (return (`SceneComponent.K2_GetComponentLocation` (`Actor.RootComponent` (`self.CurrentTarget`))))
        (else
          (for _array_element (`self.PlayerCars`)
            (if (!= (`local.Player`) _array_element)
              (if (> (`/Game/DeliveryDriver/Core/Player/BP_BasePlayerCar.CurrentDeliveryParts` _array_element) 0)
                (`/Game/DeliveryDriver/Core/Player/BP_BasePlayerCar.SetDirectionArrowColor` (`local.Player`) true true)
                (return (`SceneComponent.K2_GetComponentLocation` (`Actor.RootComponent` _array_element)))
                (else
                  (bind _outactors (`GameplayStatics.GetAllActorsOfClass` "/Game/DeliveryDriver/Core/Delivery/BP_BaseDelivery.BP_BaseDelivery_C"))
                  (if (> (`KismetArrayLibrary.Array_Length` _outactors) 0)
                    (`/Game/DeliveryDriver/Core/Player/BP_BasePlayerCar.SetDirectionArrowColor` (`local.Player`) true false)
                    (return (`SceneComponent.K2_GetComponentLocation` (`Actor.RootComponent` (`|GetArrayItem` _outactors))))
                    (else
                      (`KismetSystemLibrary.PrintString` "No valid Delivery Arrow Target Found!" true true (struct :`R` 1.0 :`B` 0.082829 :`A` 1.0))
                      (return (0.0 0.0 0.0)))))))))))))

(fn `NewTarget`
  (params (bMinDistance :type Boolean :default true) (MinDistanceStartPoint :type "Vector Structure"))
  (returns (OutputPin :type "/Game/DeliveryDriver/Core/Delivery/BP_BaseDeliveryTarget Object Reference"))
  (locals (PosssibleTargets :type "Array of /Game/DeliveryDriver/Core/Delivery/BP_BaseDeliveryTarget Object Reference"))
  (if bMinDistance
    (for _array_element (`self.DeliverytTargets`)
      (if (> (`KismetMathLibrary.Vector_Distance` (`SceneComponent.K2_GetComponentLocation` (`Actor.RootComponent` _array_element)) MinDistanceStartPoint) (`self.MinDeliveryDistance`))
        (`KismetArrayLibrary.Array_Add` (`local.PosssibleTargets`) _array_element)))
    (if (> (`KismetArrayLibrary.Array_Length` (`local.PosssibleTargets`)) 0)
      (return (`KismetArrayLibrary.Array_Random` (`local.PosssibleTargets`)))
      (else
        _)))
  (bind _outitem (`KismetArrayLibrary.Array_Random` (`self.DeliverytTargets`)))
  (return _outitem))

(fn `StartDelivery`
  (params (PlayerID :type Integer))
  (returns (Target :type "/Game/DeliveryDriver/Core/Delivery/BP_BaseDeliveryTarget Object Reference"))
  (`KismetSystemLibrary.PrintString` (`KismetStringLibrary.Concat_StrStr` "Started Delivery for Player: " (`KismetStringLibrary.Conv_IntToString` PlayerID)))
  (return null))

(fn `UserConstructionScript`)