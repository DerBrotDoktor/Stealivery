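; Base delivery pickup actor that the player car collects by driving into it to start a delivery.
; A tick after BeginPlay it enables overlaps on its collect area and registers with the minimap camera.
; The first player car overlap passes delivery data and parts to the car and reports any valid target to the delivery manager.
; It then hides mesh and minimap indicator, plays effects and destroys itself after the VFX length.
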(event `self.ReceiveBeginPlay`
  ;[0.6 0.15 0.15 0.5] Begin Play
  (`KismetSystemLibrary.DelayUntilNextTick`)
  (set `PrimitiveComponent.bGenerateOverlapEvents` true (`self.CollectArea`))
  (bind _returnvalue (`GameplayStatics.GetActorOfClass` "/Game/DeliveryDriver/UI/MiniMap/BP_MiniMapCamera.BP_MiniMapCamera_C"))
  (`/Engine/EditorBlueprintResources/StandardMacros.IsValid` _returnvalue
    (:`Is Valid`
      (`/Game/DeliveryDriver/UI/MiniMap/BP_MiniMapCamera.AddToDisplay` _returnvalue self))))

(event `self.CollectArea.OnComponentBeginOverlap`
  (params (OverlappedComponent :type "PrimitiveComponent Object Reference") (OtherActor :type "Actor Object Reference") (OtherComp :type "PrimitiveComponent Object Reference") (OtherBodyIndex :type Integer) (bFromSweep :type Boolean) (SweepResult :type "HitResult Structure (by ref)"))
  (bind _target (break `/Game/DeliveryDriver/Core/Delivery/SDeliveryData` (`self.Data`)))
  ; Pick Up
  (bind _asbp_base_player_car (cast `/Game/DeliveryDriver/Core/Player/BP_BasePlayerCar` OtherActor))
  (`/Engine/EditorBlueprintResources/StandardMacros.DoOnce` false
    (:`Completed`
      (`/Game/DeliveryDriver/Core/Player/BP_BasePlayerCar.StartDelivery` _asbp_base_player_car (`self.Data`) (`self.DeliveryParts`))
      (bind _returnvalue (`GameplayStatics.GetActorOfClass` "/Game/DeliveryDriver/Core/Delivery/BP_DeliveryManager.BP_DeliveryManager_C"))
      (`/Engine/EditorBlueprintResources/StandardMacros.IsValid` _target
        (:`Is Valid`
          (`/Game/DeliveryDriver/Core/Delivery/BP_DeliveryManager.OnDeliveryCollected` _returnvalue _target))
        (:`Is Not Valid`
          _))
      (`SceneComponent.SetVisibility` (`self.Mesh`) false false)
      (`ActorComponent.Activate` (`self.PickUpVFX`) false)
      (`AudioComponent.Play` (`self.PickUpSFX`) 0.0)
      (`GameplayStatics.GetActorOfClass` "/Game/DeliveryDriver/UI/MiniMap/BP_MiniMapCamera.BP_MiniMapCamera_C")
      (`SceneComponent.SetVisibility` (`self.MiniMapIndicator`) false false)
      (`KismetSystemLibrary.Delay` (`self.VFXLength`))
      (`self.K2_DestroyActor`))))

(fn `UserConstructionScript`)