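; Base delivery drop-off target that completes a player car's delivery when that car drives into its area.
; Starts disabled; Enable shows a colored beam and minimap indicator.
; On overlap, if the car's current target is this actor, it plays success effects, passes the parts to BP_DeliveryManager, adds score through the game instance and updates the HUD.
; The car then finishes its delivery, and the target disables itself if DeliverParts returns true.
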(event `self.ReceiveBeginPlay`
  (`self.Disable`)
  (bind _returnvalue (`GameplayStatics.GetActorOfClass` "/Game/DeliveryDriver/Core/Delivery/BP_DeliveryManager.BP_DeliveryManager_C"))
  (set `self.DeliverManager` _returnvalue))

(event `self.Area.OnComponentBeginOverlap`
  (params (OverlappedComponent :type "PrimitiveComponent Object Reference") (OtherActor :type "Actor Object Reference") (OtherComp :type "PrimitiveComponent Object Reference") (OtherBodyIndex :type Integer) (bFromSweep :type Boolean) (SweepResult :type "HitResult Structure (by ref)"))
  (bind _successvfx (`self.SuccessVFX`))
  (bind _asbp_base_player_car (cast `/Game/DeliveryDriver/Core/Player/BP_BasePlayerCar` OtherActor))
  (bind _currentdelivery_target (break `/Game/DeliveryDriver/Core/Delivery/SDeliveryData` (`/Game/DeliveryDriver/Core/Player/BP_BasePlayerCar.CurrentDelivery` _asbp_base_player_car)))
  (if (== _currentdelivery_target self)
    (`NiagaraComponent.ResetSystem` _successvfx)
    (`ActorComponent.Activate` _successvfx false)
    (`AudioComponent.Play` (`self.DeliverySuccess_SFX`) 0.0)
    (bind _currentdeliveryparts (`/Game/DeliveryDriver/Core/Player/BP_BasePlayerCar.CurrentDeliveryParts` _asbp_base_player_car))
    (bind _deliverycompleted (`/Game/DeliveryDriver/Core/Delivery/BP_DeliveryManager.DeliverParts` (`self.DeliverManager`) _currentdeliveryparts))
    (bind _playerid (`/Game/DeliveryDriver/Core/Player/BP_BasePlayerCar.PlayerID` _asbp_base_player_car))
    (`KismetSystemLibrary.PrintString` (`KismetStringLibrary.Concat_StrStr` "Finished Delivery for Player: " (`KismetStringLibrary.Conv_IntToString` _playerid)))
    (bind _asgi_game_instance (cast `/Game/DeliveryDriver/Core/Game/GI_GameInstance` (`GameplayStatics.GetGameInstance`)))
    (bind _newscore (`/Game/DeliveryDriver/Core/Game/GI_GameInstance.AddScore` _asgi_game_instance _currentdeliveryparts _playerid))
    ; Player HUD
    (`/Engine/EditorBlueprintResources/StandardMacros.IsValid` (`self.PlayerHUD`)
      (:`Is Valid`
        _)
      (:`Is Not Valid`
        (bind _foundwidgets (`WidgetBlueprintLibrary.GetAllWidgetsOfClass` "/Game/DeliveryDriver/UI/WBP_PlayerHUD.WBP_PlayerHUD_C"))
        (set `self.PlayerHUD` (`|GetArrayItem` _foundwidgets))))
    (`/Game/DeliveryDriver/UI/WBP_PlayerHUD.SetScore` (`self.PlayerHUD`) _playerid _newscore)
    (`/Game/DeliveryDriver/Core/Player/BP_BasePlayerCar.FinishDelivery` _asbp_base_player_car)
    (if _deliverycompleted
      (`self.Disable`))))

(fn `Disable`
  (`SceneComponent.SetVisibility` (`self.BeamVFX`) false false)
  (`ActorComponent.SetActive` (`self.Area`) false false)
  (`SceneComponent.SetVisibility` (`self.MiniMapIndicator`) false false)
  (set `self.bEnabled` false)
  (return))

(fn `Enable`
  (params (Color :type "LinearColor Structure"))
  (`FXSystemComponent.SetColorParameter` (`self.BeamVFX`) "Color" Color)
  (`NiagaraComponent.ResetSystem` (`self.BeamVFX`))
  (`SceneComponent.SetVisibility` (`self.BeamVFX`) true false)
  (`ActorComponent.SetActive` (`self.Area`) true false)
  (`ActorComponent.Deactivate` (`self.SuccessVFX`))
  (`SceneComponent.SetVisibility` (`self.MiniMapIndicator`) true false)
  (set `self.bEnabled` true)
  (return))

(fn `UserConstructionScript`)