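; BP_BaseDeliverySpawn is a delivery pickup point that spawns an item bound for a given target.
; On BeginPlay it disables itself, deactivating its area and hiding its effects, and caches BP_DeliveryManager.
; Enable shows a color-tinted beam and pickup VFX, then spawns the configured item class at the root's location, passing it the manager's delivery parts and the target data.
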(event `self.ReceiveBeginPlay`
  (`self.Disable`)
  (bind _returnvalue (`GameplayStatics.GetActorOfClass` "/Game/DeliveryDriver/Core/Delivery/BP_DeliveryManager.BP_DeliveryManager_C"))
  (set `self.DeliveryManager` _returnvalue))

(fn `Disable`
  (`ActorComponent.SetActive` (`self.Area`) false false)
  (`SceneComponent.SetVisibility` (`self.BeamVFX`) false false)
  (`SceneComponent.SetVisibility` (`self.NS_DeliveryPickup`) false false)
  (return))

(fn `Enable`
  (params (Color :type "LinearColor Structure") (DeliveryTarget :type "/Game/DeliveryDriver/Core/Delivery/BP_BaseDeliveryTarget Object Reference"))
  ; Beam VFX
  (`FXSystemComponent.SetColorParameter` (`self.BeamVFX`) "Color" Color)
  (`NiagaraComponent.ResetSystem` (`self.BeamVFX`))
  (`SceneComponent.SetVisibility` (`self.BeamVFX`) true false)
  (`NiagaraComponent.ResetSystem` (`self.NS_DeliveryPickup`))
  (`SceneComponent.SetVisibility` (`self.NS_DeliveryPickup`) true false)
  (`KismetSystemLibrary.PrintString` (`KismetStringLibrary.Concat_StrStr` "Enabled " (`KismetSystemLibrary.GetDisplayName` self)) true true (struct :`G` 1.0 :`B` 0.149541 :`A` 1.0))
  (bind _returnvalue (`|SpawnActorFromClass` (`self.DeliveryItemBP`) (`KismetMathLibrary.MakeTransform` (`SceneComponent.K2_GetComponentLocation` (`self.DefaultSceneRoot`))) "Undefined" "MultiplyWithRoot" null (struct) null))
  (set `/Game/DeliveryDriver/Core/Delivery/BP_BaseDelivery.DeliveryParts` (`/Game/DeliveryDriver/Core/Delivery/BP_DeliveryManager.DeliveryParts` (`self.DeliveryManager`)) _returnvalue)
  (set `/Game/DeliveryDriver/Core/Delivery/BP_BaseDelivery.Data` (make `/Game/DeliveryDriver/Core/Delivery/SDeliveryData` DeliveryTarget (`self.DeliveryItemBP`)) _returnvalue)
  (return))

(fn `UserConstructionScript`)