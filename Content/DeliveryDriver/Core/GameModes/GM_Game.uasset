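; Game mode for the delivery driver game that sets up local splitscreen multiplayer for player cars.
; One tick after BeginPlay, it enables splitscreen and loops over NumPlayers, creating any missing local controllers.
; Each controller gets the car input mapping, a spawned default pawn at the PlayerStart matching its index, and a player ID.
; ChoosePlayerStart is overridden to pick a start by the spawned-player count.
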(event `self.ReceiveBeginPlay`
  (bind _returnvalue (`GameplayStatics.GetPlayerController` 0))
  (bind _returnvalue_2 (`GameplayStatics.GetPlayerController` (`self.NumSpawnedPlayers`)))
  (bind _returnvalue_3 (`GameplayStatics.GetPlayerController` (`self.NumSpawnedPlayers`)))
  (`KismetSystemLibrary.DelayUntilNextTick`)
  (`GameplayStatics.SetForceDisableSplitscreen` false)
  (bind _outactors (`GameplayStatics.GetAllActorsOfClass` "/Script/Engine.PlayerStart"))
  (for _ (range 1 (+ (`self.NumPlayers`) 1))
    (`/Engine/EditorBlueprintResources/StandardMacros.IsValid` _returnvalue_2
      (:`Is Valid`
        _)
      (:`Is Not Valid`
        (`GameplayStatics.CreatePlayer` -1)))
    (`WidgetBlueprintLibrary.SetInputMode_GameAndUIEx` _returnvalue_2 null)
    (if (> (`self.NumSpawnedPlayers`) 0)
      (`EnhancedInputSubsystemInterface.AddMappingContext` (pcsubsystem `EnhancedInputLocalPlayerSubsystem` _returnvalue_2) "/Game/DeliveryDriver/Player/Input/IMC_PlayerCar.IMC_PlayerCar" 0 (struct))
      (bind _returnvalue_4 (`self.GetTransform` (`|GetArrayItem` _outactors (`self.NumSpawnedPlayers`))))
      (bind _returnvalue_5 (`|SpawnActorFromClass` (`self.DefaultPlayerClass`) _returnvalue_4 "Undefined" "MultiplyWithRoot" null null))
      (`Controller.Possess` _returnvalue_3 _returnvalue_5)
      (bind _aspc_player_car (cast `/Game/DeliveryDriver/Core/Player/PC_PlayerCar` _returnvalue_3))
      (`/Game/DeliveryDriver/Core/Player/PC_PlayerCar.SetPlayerID` _aspc_player_car (`self.NumSpawnedPlayers`))
      (`/Engine/EditorBlueprintResources/StandardMacros.IncrementInt` (`self.NumSpawnedPlayers`))
      (else
        (`EnhancedInputSubsystemInterface.AddMappingContext` (pcsubsystem `EnhancedInputLocalPlayerSubsystem` _returnvalue) "/Game/DeliveryDriver/Player/Input/IMC_PlayerCar.IMC_PlayerCar" 0 (struct))
        (bind _returnvalue_6 (`|SpawnActorFromClass` (`self.DefaultPlayerClass`) _returnvalue_4 "Undefined" "MultiplyWithRoot" null null))
        (`Controller.Possess` _returnvalue _returnvalue_6)
        (bind _aspc_player_car_2 (cast `/Game/DeliveryDriver/Core/Player/PC_PlayerCar` _returnvalue))
        (`/Game/DeliveryDriver/Core/Player/PC_PlayerCar.SetPlayerID` _aspc_player_car_2 (`self.NumSpawnedPlayers`))
        (`/Engine/EditorBlueprintResources/StandardMacros.IncrementInt` (`self.NumSpawnedPlayers`))))))

(fn `ChoosePlayerStart`
  (params (Player :type "Controller Object Reference"))
  (returns (ReturnValue :type "Actor Object Reference"))
  (bind _outactors (`GameplayStatics.GetAllActorsOfClass` "/Script/Engine.PlayerStart"))
  (return (`|GetArrayItem` _outactors (`KismetMathLibrary.Clamp` (`self.NumSpawnedPlayers`) 0 (`KismetArrayLibrary.Array_Length` _outactors)))))

(fn `UserConstructionScript`)