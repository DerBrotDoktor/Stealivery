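; Player-controlled delivery car that layers character visuals, audio and feedback onto its parent vehicle class.
; On initialization it picks the driver mesh and minimap icon from the GameInstance's per-player character choice and offsets a spring arm by PlayerID.
; Throttle and brake input drive ABP_Player flags, with throttle also swapping large and small exhaust smoke.
; Low-speed hits and finished deliveries play crash and celebrate montages, and honk input plays a sound.
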(event `self.OnInitializePlayer`
  ;[0.6 0.15 0.15 0.5] Initialize Player
  (`parent.OnInitializePlayer`)
  (`KismetSystemLibrary.DelayUntilNextTick`)
  (bind _asgi_game_instance (cast `/Game/DeliveryDriver/Core/Game/GI_GameInstance` (`GameplayStatics.GetGameInstance`)))
  (bind _output (`|GetArrayItem` (`/Game/DeliveryDriver/Core/Game/GI_GameInstance.CharacterIndexs` _asgi_game_instance) (`self.PlayerID`)))
  (`SkeletalMeshComponent.SetSkeletalMeshAsset` (`self.CharacterMesh`) (`|GetArrayItem` (`self.CharacterMeshs`) _output))
  (`PaperSpriteComponent.SetSprite` (`self.MiniMapInidicatorCharacter`) (`|GetArrayItem` (`self.CharacterMiniMapIndicators`) _output))
  (`SceneComponent.K2_AddLocalOffset` (`self.SpringArm2`) (`KismetMathLibrary.MakeVector` 0.0 0.0 (`KismetMathLibrary.Conv_IntToDouble` (* (`self.PlayerID`) 5))) false false))

(event `self.ReceiveBeginPlay`
  ;[0.6 0.15 0.15 0.5] Begin Play
  (`parent.ReceiveBeginPlay`)
  (`ActorComponent.SetActive` (`self.NS_Smoke_Right`) false false)
  (bind _asabp_player (cast `/Game/DeliveryDriver/Characters/PlayerAnimations/ABP_Player` (`SkeletalMeshComponent.GetAnimInstance` (`self.CharacterMesh`))))
  (set `self.CharacterAnimInstance` _asabp_player)
  (`self.EnableSmallSmokeVFX`))

(event `EnhancedInput|/Game/DeliveryDriver/Player/Input/Actions/IA_Throttle`
  (params (ActionValue :type "Float (double-precision)") (ElapsedSeconds :type "Float (double-precision)") (TriggeredSeconds :type "Float (double-precision)") (InputAction :type "InputAction Object Reference" :default "/Game/DeliveryDriver/Player/Input/Actions/IA_Throttle.IA_Throttle"))
  ; Smoke VFX
  (:`Started`
    (`self.EnableSmokeVFX`)
    (set `/Game/DeliveryDriver/Characters/PlayerAnimations/ABP_Player.bAccelerating` true (`self.CharacterAnimInstance`)))
  (:`Canceled`
    (`self.EnableSmallSmokeVFX` :!label _label)
    (set `/Game/DeliveryDriver/Characters/PlayerAnimations/ABP_Player.bAccelerating` false (`self.CharacterAnimInstance`)))
  (:`Completed`
    (goto _label)))

(event `EnableSmokeVFX`
  ; Smoke VFX
  (`ActorComponent.SetActive` (`self.NS_Smoke_Right`) true false)
  (`ActorComponent.SetActive` (`self.NS_SmallSmoke_Right`) false false)
  (`ActorComponent.SetActive` (`self.NS_Smoke_Left`) true false)
  (`ActorComponent.SetActive` (`self.NS_SmallSmoke_Left`) false false))

(event `EnableSmallSmokeVFX`
  ; Smoke VFX
  (`ActorComponent.SetActive` (`self.NS_Smoke_Right`) false false)
  (`ActorComponent.SetActive` (`self.NS_SmallSmoke_Right`) true false)
  (`ActorComponent.SetActive` (`self.NS_Smoke_Left`) false false)
  (`ActorComponent.SetActive` (`self.NS_SmallSmoke_Left`) true false))

(event `EnhancedInput|/Game/DeliveryDriver/Player/Input/Actions/IA_Brake`
  (params (ActionValue :type "Float (double-precision)") (ElapsedSeconds :type "Float (double-precision)") (TriggeredSeconds :type "Float (double-precision)") (InputAction :type "InputAction Object Reference" :default "/Game/DeliveryDriver/Player/Input/Actions/IA_Brake.IA_Brake"))
  ; Break
  (:`Started`
    (set `/Game/DeliveryDriver/Characters/PlayerAnimations/ABP_Player.bBreaking` true (`self.CharacterAnimInstance`)))
  (:`Canceled`
    (set `/Game/DeliveryDriver/Characters/PlayerAnimations/ABP_Player.bBreaking` false (`self.CharacterAnimInstance`) :!label _label_2))
  (:`Completed`
    (goto _label_2)))

(event `EnhancedInput|/Game/DeliveryDriver/Player/Input/Actions/AI_Honk`
  (params (ActionValue :type Boolean) (ElapsedSeconds :type "Float (double-precision)") (TriggeredSeconds :type "Float (double-precision)") (InputAction :type "InputAction Object Reference" :default "/Game/DeliveryDriver/Player/Input/Actions/AI_Honk.AI_Honk"))
  ; Honk
  (:`Completed`
    (`AudioComponent.Play` (`self.HonkSFX`) 0.0)))

(event `self.OnHit`
  ; Hit
  (`parent.OnHit`)
  (if (< (`KismetMathLibrary.VSize` (`self.GetVelocity`)) 50.0)
    (`AnimInstance.Montage_Play` (`self.CharacterAnimInstance`) "/Game/DeliveryDriver/Characters/PlayerAnimations/AM_Crash_Montage.AM_Crash_Montage" 1.0 "MontageLength" 0.0 true)))

(event `SetMiniMapIcons`
  ; Mini Map
  (`PaperSpriteComponent.SetSprite` (`self.MiniMapInidicator`) (`|GetArrayItem` (`self.MiniMapDirectionSprites`) (`self.PlayerID`))))

(fn `FinishDelivery`
  (`parent.FinishDelivery`)
  (`AnimInstance.Montage_Play` (`self.CharacterAnimInstance`) "/Game/DeliveryDriver/Characters/PlayerAnimations/AM_Celebrate_Montage.AM_Celebrate_Montage" 1.0 "MontageLength" 0.0 true))

(fn `UserConstructionScript`
  (`SceneComponent.K2_AttachToComponent` (`self.DeliveryMesh`) (`self.Mesh`) "DeliverySocket" "KeepWorld" "KeepWorld" "KeepWorld" true))