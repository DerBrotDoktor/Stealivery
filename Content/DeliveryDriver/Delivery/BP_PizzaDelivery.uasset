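; BP_PizzaDelivery is a pizza delivery actor in the Delivery Driver game with an animated mesh and a collect area.
; On BeginPlay it starts a Timeline that drives the mesh's relative height and yaw.
; A one-second timer then enables query-only collision on CollectArea, delaying when it can be collected.
; Collection handling is not in this graph; BeginPlay also calls the parent implementation.
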(event `self.ReceiveBeginPlay`
  (bind (_relativerotation_roll _relativerotation_pitch) (`KismetMathLibrary.BreakRotator` (`SceneComponent.RelativeRotation` (`self.Mesh`))))
  (bind (_relativelocation_x _relativelocation_y) (`KismetMathLibrary.BreakVector` (`SceneComponent.RelativeLocation` (`self.Mesh`))))
  (`parent.ReceiveBeginPlay`)
  (`KismetSystemLibrary.K2_SetTimerDelegate` (delegate `EnableCollect`) 1.0)
  (bind (_direction _position _rotation) (`Timeline|Timeline`)
    (:`Update`
      (`SceneComponent.K2_SetRelativeLocation` (`self.Mesh`) (`KismetMathLibrary.MakeVector` _relativelocation_x _relativelocation_y _position) false false)
      (`SceneComponent.K2_SetRelativeRotation` (`self.Mesh`) (`KismetMathLibrary.MakeRotator` _relativerotation_roll _relativerotation_pitch _rotation) false false))))

(event `EnableCollect`
  (`PrimitiveComponent.SetCollisionEnabled` (`self.CollectArea`) "QueryOnly"))

(fn `UserConstructionScript`
  (`parent.UserConstructionScript`))