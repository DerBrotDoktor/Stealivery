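; BP_NPCCharacter is a Mass-driven pedestrian NPC that gets a random skeletal mesh and material on BeginPlay and reacts to being hit by the player's car.
; A capsule hit from an IPlayerCar actor applies a scaled-down impulse to the mesh and plays NPCHit, once only.
; OnPlayerBumped stops movement and enables physics on mesh and capsule once, then destroys the Mass entity after a delay.
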(event `self.ReceiveBeginPlay`
  (`SkeletalMeshComponent.SetSkeletalMeshAsset` (`self.Mesh`) (`KismetArrayLibrary.Array_Random` (`self.Meshs`)))
  (`PrimitiveComponent.SetMaterial` (`self.Mesh`) 0 (`KismetArrayLibrary.Array_Random` (`self.Materials`))))

(event `self.CapsuleComponent.OnComponentHit`
  (params (HitComponent :type "PrimitiveComponent Object Reference") (OtherActor :type "Actor Object Reference") (OtherComp :type "PrimitiveComponent Object Reference") (NormalImpulse :type "Vector Structure") (Hit :type "HitResult Structure (by ref)"))
  (if (`KismetSystemLibrary.DoesImplementInterface` OtherActor "/Game/DeliveryDriver/Core/Player/IPlayerCar.IPlayerCar_C")
    (`/Engine/EditorBlueprintResources/StandardMacros.DoOnce` false
      (:`Completed`
        (`PrimitiveComponent.AddImpulse` (`self.Mesh`) (/ NormalImpulse 7.0) "None" true)
        (`AudioComponent.Play` (`self.NPCHit`) 0.0)))))

(event `/Game/DeliveryDriver/Core/Enviroment/IBumpable.OnPlayerBumped`
  (`/Engine/EditorBlueprintResources/StandardMacros.DoOnce` false
    (:`Completed`
      (`KismetSystemLibrary.PrintString` "NPC Bumped")
      (`PrimitiveComponent.SetSimulatePhysics` (`self.Mesh`) true)
      (`MovementComponent.StopMovementImmediately` (`self.CharacterMovement`))
      (`PrimitiveComponent.SetSimulatePhysics` (`self.CapsuleComponent`) true)
      (`KismetSystemLibrary.Delay` 10.0)
      (`NPCMassAgentComponent.DestroyMassEntity` (`self.NPCMassAgent`)))))

(fn `UserConstructionScript`)