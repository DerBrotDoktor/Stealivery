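; BP_Trashcan is a physics prop trashcan for the delivery driver game that bursts trash when the player bumps it.
; Its OnPlayerBumped event spawns the NS_Burst_Trash effect at the mesh's world location, raised slightly upward.
; The graph only responds to that event; bump detection happens outside it, and the construction script just calls the parent.
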(event `/Game/DeliveryDriver/Core/Enviroment/IBumpable.OnPlayerBumped`
  (`NiagaraFunctionLibrary.SpawnSystemAtLocation` "/Game/DeliveryDriver/Effects/Burst/NS_Burst_Trash.NS_Burst_Trash" (+ (`SceneComponent.K2_GetComponentLocation` (`self.Mesh`)) (0.0 0.0 50.0))))

(fn `UserConstructionScript`
  (`parent.UserConstructionScript`))