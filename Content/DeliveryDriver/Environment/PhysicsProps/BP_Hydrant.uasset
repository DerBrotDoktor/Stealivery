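; BP_Hydrant is a fire hydrant physics prop that spawns a water fountain when a Pawn hits it.
; The mesh's hit event passes through a DoOnce gate, then casts the other actor to Pawn.
; A successful cast spawns BP_WaterFountain at the mesh's current world location, while a failed one resets the gate, so only the first Pawn hit triggers the fountain.
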(event `self.Mesh.OnComponentHit`
  (params (HitComponent :type "PrimitiveComponent Object Reference") (OtherActor :type "Actor Object Reference") (OtherComp :type "PrimitiveComponent Object Reference") (NormalImpulse :type "Vector Structure") (Hit :type "HitResult Structure (by ref)"))
  (`/Engine/EditorBlueprintResources/StandardMacros.DoOnce` false :!label _label
    (:`Completed`
      (cast `Pawn` OtherActor
        (:`then`
          (`|SpawnActorFromClass` "/Game/DeliveryDriver/Effects/WaterFountain/BP_WaterFountain.BP_WaterFountain_C" (`KismetMathLibrary.MakeTransform` (`SceneComponent.K2_GetComponentLocation` (`self.Mesh`))) "AlwaysSpawn" "MultiplyWithRoot" null null))
        (:`CastFailed`
          (goto _label :!via `Reset`))))))

(fn `UserConstructionScript`
  (`parent.UserConstructionScript`))