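; BP_BusStation is a destructible bus station prop that breaks apart after a player car reaches it.
; A box overlap with an IPlayerCar actor enables physics, gravity and collision damage on its Geometry Collection, once.
; The same overlap opens a closed DoOnce gate, so only a later Chaos break event counts.
; The first counted break prints a debug string and destroys the actor after a delay.
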(event `self.GeometryCollectionComponent.OnChaosBreakEvent`
  (params (BreakEvent :type "ChaosBreakEvent Structure (by ref)"))
  (`/Engine/EditorBlueprintResources/StandardMacros.DoOnce` true :!label _label
    (:`Completed`
      (`KismetSystemLibrary.PrintString` "break")
      (`KismetSystemLibrary.Delay` 15.0)
      (`self.K2_DestroyActor`))))

(event `self.Box.OnComponentBeginOverlap`
  (params (OverlappedComponent :type "PrimitiveComponent Object Reference") (OtherActor :type "Actor Object Reference") (OtherComp :type "PrimitiveComponent Object Reference") (OtherBodyIndex :type Integer) (bFromSweep :type Boolean) (SweepResult :type "HitResult Structure (by ref)"))
  (bind _geometrycollectioncomponent (`self.GeometryCollectionComponent`))
  (if (`KismetSystemLibrary.DoesImplementInterface` OtherActor "/Game/DeliveryDriver/Core/Player/IPlayerCar.IPlayerCar_C")
    (`/Engine/EditorBlueprintResources/StandardMacros.DoOnce` false
      (:`Completed`
        (`PrimitiveComponent.SetSimulatePhysics` _geometrycollectioncomponent true)
        (`GeometryCollectionComponent.SetEnableDamageFromCollision` _geometrycollectioncomponent true)
        (`PrimitiveComponent.SetEnableGravity` _geometrycollectioncomponent true)
        (goto _label :!via `Reset`)))))

(fn `UserConstructionScript`)